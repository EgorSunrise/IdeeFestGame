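; Treasure chest Blueprint that reveals itself with an animated movement and then signals completion of a game event.
; RevealChest, if IsActive is set, makes the chest mesh visible and fires VisibilityTriggered, returning IsActive either way.
; The ChestAnimation timeline applies additive Z movement to the root and pitch/yaw rotation to the chest, adding a Niagara component on every update.
; One second after it finishes, CallOnCompleteGameEvent runs.
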(event `VisibilityTriggered`
  (bind (_direction _changelocation _changerotationy _changerotationz) (`Timeline|ChestAnimation`)
    (:`Update`
      (`SceneComponent.K2_AddRelativeLocation` (`self.DefaultSceneRoot`) (`KismetMathLibrary.MakeVector` 0.0 0.0 _changelocation) false false)
      (`SceneComponent.K2_AddRelativeRotation` (`self.ChestObject`) (`KismetMathLibrary.MakeRotator` 0.0 _changerotationy _changerotationz) false false)
      (`AddComponent|NODE_AddNiagaraComponent-0`))
    (:`Finished`
      (`KismetSystemLibrary.Delay` 1.0)
      (`self.OnCompleteGameEvent`))))

(fn `RevealChest`
  (returns (Success :type Boolean))
  (bind _isactive (`self.isActive`))
  (if _isactive
    (`SceneComponent.SetVisibility` (`self.ChestObject`) true false)
    (`self.VisibilityTriggered`))
  (return _isactive))

(fn `UserConstructionScript`)