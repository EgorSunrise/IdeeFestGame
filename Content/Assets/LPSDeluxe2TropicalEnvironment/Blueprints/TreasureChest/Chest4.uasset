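; Chest4 is a treasure chest Blueprint that reveals itself when BP_Player overlaps its Sphere.
; RevealChest makes ChestObject visible, then triggers the ChestAnimation timeline, whose values are added each update as relative Z movement plus pitch and yaw rotation.
; Every overlap also adds a Control Rig component before the player cast, so any overlapping actor causes this, and nothing uses that component.
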(event `VisibilityTriggered`
  (bind (_direction _changelocation _changerotationy _changerotationz) (`Timeline|ChestAnimation`)
    (:`Update`
      (`SceneComponent.K2_AddRelativeLocation` (`self.ChestObject`) (`KismetMathLibrary.MakeVector` 0.0 0.0 _changelocation) false false)
      (`SceneComponent.K2_AddRelativeRotation` (`self.ChestObject`) (`KismetMathLibrary.MakeRotator` 0.0 _changerotationy _changerotationz) false false))))

(event `self.Sphere.OnComponentBeginOverlap`
  (params (OverlappedComponent :type "PrimitiveComponent Object Reference") (OtherActor :type "Actor Object Reference") (OtherComp :type "PrimitiveComponent Object Reference") (OtherBodyIndex :type Integer) (bFromSweep :type Boolean) (SweepResult :type "HitResult Structure (by ref)"))
  (`AddComponent|NODE_AddControlRigComponent-0`)
  (cast `/Game/Blueprints/Player/BP_Player` OtherActor)
  (`self.RevealChest`))

(fn `RevealChest`
  (`SceneComponent.SetVisibility` (`self.ChestObject`) true false)
  (`self.VisibilityTriggered`))

(fn `UserConstructionScript`)