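; GM_TreasureHuntMode is the game mode for a treasure hunt in which one randomly chosen chest holds the objective.
; On BeginPlay it gathers all Chest actors, activates one at random, passes it to BP_Player as the treasure actor and binds to its OnCompleteGameEvent.
; On completion, it moves player control to a placed BP_CompleteGamePawn and starts the crown animation on the ChestOpen actor.
; An unconnected player teleport node never runs.
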(event `self.ReceiveBeginPlay`
  (bind _outactors (`GameplayStatics.GetAllActorsOfClass` "/Game/Assets/LPSDeluxe2TropicalEnvironment/Blueprints/TreasureChest/Chest.Chest_C"))
  (bind _output_get (set `self.TreasureChestArray` _outactors))
  (bind _index (`self.GetRandomIndex` _output_get))
  (bind _output (`|GetArrayItem` _output_get _index))
  (set `/Game/Assets/LPSDeluxe2TropicalEnvironment/Blueprints/TreasureChest/Chest.isActive` true _output)
  (bind _asbp_player (cast `/Game/Blueprints/Player/BP_Player` (`GameplayStatics.GetPlayerCharacter` 0)))
  (`/Game/Blueprints/Player/BP_Player.SetTreasureActor` _asbp_player _output)
  (add `/Game/Assets/LPSDeluxe2TropicalEnvironment/Blueprints/TreasureChest/Chest.OnCompleteGameEvent` _output (delegate `CompleteGame`)))

(event `CompleteGame`
  (bind _returnvalue (`GameplayStatics.GetPlayerController` 0))
  (`Controller.UnPossess` _returnvalue)
  (bind _outactors (`GameplayStatics.GetAllActorsOfClass` "/Game/Blueprints/Player/BP_CompleteGamePawn.BP_CompleteGamePawn_C"))
  (`Controller.Possess` _returnvalue (`|GetArrayItem` _outactors))
  (bind _outactors_2 (`GameplayStatics.GetAllActorsOfClass` "/Game/Assets/LPSDeluxe2TropicalEnvironment/Blueprints/TreasureChest/ChestOpen.ChestOpen_C"))
  (`/Game/Assets/LPSDeluxe2TropicalEnvironment/Blueprints/TreasureChest/ChestOpen.StartCrownAnim` (`|GetArrayItem` _outactors_2)))

(fn `GetRandomIndex`
  (params (ActorArray :type "Array of Actor Object Reference"))
  (returns (Index :type Integer))
  (return (`KismetMathLibrary.RandomIntegerInRange` 0 (- (`KismetArrayLibrary.Array_Length` ActorArray) 1))))

(fn `UserConstructionScript`)